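; Blueprint function that turns the player's control rotation toward the point under the mouse cursor and shifts the camera toward it.
; When the Visibility cursor trace returns a non-zero impact normal, it sets a look-at rotation from the pawn through RInterpTo, whose zero speed makes it instant.
; The passed-in spring arm's horizontal TargetOffset lerps by the timeline input toward half the pawn-to-cursor vector, clamped in length.
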(fn AimtoCrossHair
  (params (TimelinIn :type Float%20%28single-precision%29%20%28by%20ref%29) (SpringArm :type Spring%20Arm%20Component%20Object%20Reference%20%28by%20ref%29))
  (bind _returnvalue (Game|GetPlayerController 0))
  (bind _hitresult (Game|Player|GetHitResultUnderCursorbyChannel _returnvalue "TraceTypeQuery1" true))
  (bind _returnvalue_2 (Pawn|GetControlledPawn _returnvalue))
  (bind (_bblockinghit _binitialoverlap _time _distance _location _impactpoint _normal _impactnormal) (Collision|BreakHitResult _hitresult))
  (bind _returnvalue_3 (Transformation|GetActorLocation _returnvalue_2))
  (LocalVariables|SetTI TimelinIn)
  (LocalVariables|SetSA SpringArm)
  (if (not (Math|Vector|Equal(Vector) _impactnormal "0, 0, 0" 0.0001))
    (Pawn|SetControlRotation _returnvalue (Math|Interpolation|RInterpTo (Math|Conversions|RotationFromXVector (Transformation|GetActorLocation _returnvalue_2)) (Math|Rotator|FindLookatRotation _returnvalue_3 _location) (Utilities|Time|GetWorldDeltaSeconds) 0.0))
    (Variables|/Script/Engine.SpringArmComponent|SetTargetOffset (LocalVariables|GetSA) (Math|Vector|MakeVector (.x (Math|Vector|Lerp(Vector) (Variables|/Script/Engine.SpringArmComponent|GetTargetOffset (LocalVariables|GetSA)) (Math|Vector|ClampVectorSize (Math|Vector|NegateVector (/ (- _returnvalue_3 _location) 2)) 0.0 2.5e+02) (LocalVariables|GetTI))) (.y (Math|Vector|Lerp(Vector) (Variables|/Script/Engine.SpringArmComponent|GetTargetOffset (LocalVariables|GetSA)) (Math|Vector|ClampVectorSize (Math|Vector|NegateVector (/ (- _returnvalue_3 _location) 2)) 0.0 2.5e+02) (LocalVariables|GetTI))) 0.0))
    (return)))