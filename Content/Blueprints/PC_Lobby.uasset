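; Lobby player controller that toggles the HUD_MenuLobby menu and manages the mouse cursor.
; Escape or the Inventory action creates the widget on first use, then adds it to or removes it from the viewport.
; The open menu uses a hand cursor, while Resume restores a crosshair cursor locked to the viewport.
; The in-game cursor setup sets Game Only input, then immediately overrides it with Game and UI.
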(event Custom|Resume
  ;[1 1 1] Fermeture Menu Echap
  (Widget|RemovefromParent (Variables|Default|GethudMenuLobby))
  (CallFunction|CursorIngame))

(event Custom|CursorMenu
  ;[1 1 1] Init Cursor
  (Input|SetInputModeGameandUI self 0 "DoNotLock" false)
  (Variables|Default|SetCurrentMouseCursor "Hand"))

(event Custom|CursorIngame
  (bind _self self)
  ;[1 1 1] Curseur en game
  (Variables|Default|SetCurrentMouseCursor "Crosshairs")
  (Input|SetInputModeGameOnly _self)
  (Input|SetInputModeGameandUI _self 0 "LockAlways" false))

(event EventBeginPlay
  (Variables|Default|SetbShowMouseCursor true)
  (CallFunction|CursorIngame))

(event Input|ActionEvents|InputActionInventory
  (params (Key :type Key%20Structure :default "None"))
  ;[1 1 1] Echap en jeu
  (:Released
    (Utilities|IsValid (Variables|Default|GethudMenuLobby)
      (:Is%20Valid
        (if (Widget|IsVisible (Variables|Default|GethudMenuLobby))
          (CallFunction|Resume)
          (else
            (UserInterface|Viewport|AddtoViewport (stale _output_get) 0 :!label _label)
            (CallFunction|CursorMenu))))
      (:Is%20Not%20Valid
        (bind _returnvalue (UserInterface|CreateWidget "/Game/HUD/HUD_MenuLobby.HUD_MenuLobby_C"))
        (bind _output_get (Variables|Default|SethudMenuLobby _returnvalue))
        (goto _label)))))

(event Input|ActionEvents|InputActionLeftClick
  (params (Key :type Key%20Structure :default "None")))

(event Input|KeyboardEvents|Escape
  (params (Key :type Key%20Structure :default "None"))
  ;[1 1 1] Echap en jeu
  (:Released
    (Utilities|IsValid (Variables|Default|GethudMenuLobby)
      (:Is%20Valid
        (if (Widget|IsVisible (Variables|Default|GethudMenuLobby))
          (CallFunction|Resume)
          (else
            (UserInterface|Viewport|AddtoViewport (stale _output_get) 0 :!label _label)
            (CallFunction|CursorMenu))))
      (:Is%20Not%20Valid
        (bind _returnvalue (UserInterface|CreateWidget "/Game/HUD/HUD_MenuLobby.HUD_MenuLobby_C"))
        (bind _output_get (Variables|Default|SethudMenuLobby _returnvalue))
        (goto _label)))))

(fn ConstructionScript)