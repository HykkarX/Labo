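; Player controller for the start menu that handles menu screens, hosting and joining multiplayer games.
; Shows the cursor, lazily creates and caches the start and multiplayer widgets, and uses Escape to quit from the start menu or return from multiplayer.
; Hosting creates a non-LAN session and opens the Lobby as a listen server.
; Joining bypasses session search, running an "open" console command built from the given IP.
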(event Custom|HUD%20-%20Multiplayer
  ;[1 1 1] HUD Menu Multiplayer
  (Utilities|IsValid (Variables|Default|GetMenu-Multi)
    (:Is%20Valid
      _)
    (:Is%20Not%20Valid
      (bind _returnvalue (UserInterface|CreateWidget "/Game/HUD/HUD_MenuMultiplayer.HUD_MenuMultiplayer_C"))
      (bind _output_get (Variables|Default|SetMenu-Multi _returnvalue))))
  (UserInterface|Viewport|AddtoViewport _output_get 0))

(event Custom|Init%20Cursor
  ;[1 1 1] Init Cursor
  (Variables|Default|SetbShowMouseCursor true)
  (Input|SetInputModeGameandUI self 0 "DoNotLock" false))

(event Custom|Héberger
  ;[1 1 1] Host
  (|Session self 4 false
    (:OnSuccess
      (Game|OpenLevel(byName) "Lobby" true "listen"))))

(event Custom|Rejoindre
  (params (IP :type String))
  ;[1 1 1] Join
  (Development|ExecuteConsoleCommand (Utilities|String|Append "open " IP) 0))

(event Custom|HUD-Start
  ;[1 1 1] HUD Menu Multiplayer
  (Utilities|IsValid (Variables|Default|GetMenu-Start)
    (:Is%20Valid
      _)
    (:Is%20Not%20Valid
      (bind _returnvalue (UserInterface|CreateWidget "/Game/HUD/HUD_MenuStart.HUD_MenuStart_C"))
      (bind _output_get (Variables|Default|SetMenu-Start _returnvalue))))
  (UserInterface|Viewport|AddtoViewport _output_get 0))

(event EventBeginPlay
  ;[1 1 1] Init
  (CallFunction|HUD-Start)
  (CallFunction|InitCursor))

(event Input|KeyboardEvents|Escape
  (params (Key :type Key%20Structure :default "None"))
  (bind _menu_multi (Variables|Default|GetMenu-Multi))
  ;[1 1 1] Echap
  (:Released
    (if (Widget|IsVisible (Variables|Default|GetMenu-Start))
      (Game|QuitGame 0 "Quit" false)
      (elif (Widget|IsVisible _menu_multi)
        (Widget|RemovefromParent _menu_multi)
        (CallFunction|HUD-Start)))))

(fn ConstructionScript)