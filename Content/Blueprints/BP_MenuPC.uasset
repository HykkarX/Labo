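; Main menu player controller that shows the menu HUD and lets the player host or join a multiplayer session.
; On BeginPlay it creates the HUD_Menu widget once, shows the cursor and sets Game and UI input.
; Héberger creates an online session, then opens the Lobby level as a listen server.
; Rejoindre joins by IP through an "open" console command, appending the address without a separator.
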(event Custom|HUD-Menu
  ;[1 1 1] HUD Menu
  (Utilities|IsValid (Variables|Default|GetHUD_Menu)
    (:Is%20Not%20Valid
      (bind _returnvalue (UserInterface|CreateWidget "/Game/Blueprints/HUD/HUD_Menu.HUD_Menu_C"))
      (bind _output_get (Variables|Default|SetHUD_Menu _returnvalue))
      (UserInterface|Viewport|AddtoViewport _output_get 0))))

(event Custom|Init%20Cursor
  ;[1 1 1] Init Cursor
  (Variables|Default|SetbShowMouseCursor true)
  (Input|SetInputModeGameandUI self 0 "DoNotLock" false))

(event Custom|Héberger
  ;[1 1 1] Host
  (|Session self 4 false
    (:OnSuccess
      (Game|OpenLevel(byName) "Lobby" true "listen"))))

(event Custom|Rejoindre
  (params (IP :type String))
  ;[1 1 1] Join
  (Development|ExecuteConsoleCommand (Utilities|String|Append "open " IP) 0))

(event EventBeginPlay
  ;[1 1 1] Init
  (CallFunction|HUD-Menu)
  (CallFunction|InitCursor))

(fn ConstructionScript)